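; BPC_HealthComp is a health component that tracks a Health value for the actor it belongs to.
; Healing and Damage functions add to or subtract from Health, clamp it between 0 and 100, and print the result for debugging.
; BeginPlay caches the owning actor, though neither function uses it, and reaching zero health triggers no further logic here.
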(event EventBeginPlay
  (Variables|Default|SetOwner (Components|GetOwner)))

(fn Healing
  (params (HealingVal :type Float%20%28double-precision%29))
  (bind _output_get (Variables|Default|SetHealth (Math|Float|Clamp(Float) (+ (Variables|Default|GetHealth) HealingVal) 0.0 1e+02)))
  (Development|PrintString (Utilities|String|Append "Health : " (Utilities|String|ToString(Float) _output_get))))

(fn Damage
  (params (DamagingVal :type Float%20%28double-precision%29))
  (bind _output_get (Variables|Default|SetHealth (Math|Float|Clamp(Float) (- (Variables|Default|GetHealth) DamagingVal) 0.0 1e+02)))
  (Development|PrintString (Utilities|String|Append "Health : " (Utilities|String|ToString(Float) _output_get))))
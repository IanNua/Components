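; BP_BoxParent is a box actor that either heals or damages the player character on touch, chosen by its HealingType setting.
; The construction script tints the cube green for healing or red for damaging through a material colour parameter.
; BeginPlay caches the third-person player character, and the box's overlap event calls Healing or Damage on that character's health component by a fixed amount.
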(event OnComponentBeginOverlap(Box)
  (params (OverlappedComponent :type Primitive%20Component%20Object%20Reference) (OtherActor :type Actor%20Object%20Reference) (OtherComp :type Primitive%20Component%20Object%20Reference) (OtherBodyIndex :type Integer) (bFromSweep :type Boolean) (SweepResult :type Hit%20Result%20Structure%20%28by%20ref%29))
  (bind _as_bp_third_person_character (Variables|Default|GetAs%20BP%20Third%20Person%20Character))
  (bind _bpc_healthcomp (Variables|/Game/ThirdPerson/Blueprints/BP_ThirdPersonCharacter.BP_ThirdPersonCharacter_C|GetBPC_HealthComp _as_bp_third_person_character))
  (if (== OtherActor _as_bp_third_person_character)
    (switch Utilities|FlowControl|Switch|SwitchonE_Healing (Variables|Default|GetHealingType)
      (:NewEnumerator0
        (Default|Healing _bpc_healthcomp 1e+01))
      (:NewEnumerator1
        (Default|Damage _bpc_healthcomp 1e+01)))))

(event EventBeginPlay
  (bind _asbp_third_person_character (Utilities|Casting|CastToBP_ThirdPersonCharacter (Game|GetPlayerCharacter 0)))
  (Variables|Default|SetAs%20BP%20Third%20Person%20Character _asbp_third_person_character))

(fn ConstructionScript
  (bind _cube (Variables|Default|GetCube))
  (switch Utilities|FlowControl|Switch|SwitchonE_Healing (Variables|Default|GetHealingType)
    (:NewEnumerator0
      (Rendering|Material|SetVectorParameterValueonMaterials _cube "ColourParam" "0.000000,1.000000,0.000000"))
    (:NewEnumerator1
      (Rendering|Material|SetVectorParameterValueonMaterials _cube "ColourParam" "1.000000,0.000000,0.000000"))))